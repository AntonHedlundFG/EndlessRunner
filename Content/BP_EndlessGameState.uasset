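; BP_EndlessGameState is the game state for an endless mode, driving the current score, high score and name entry widgets.
; BeginPlay creates the three widgets, hides name entry, and binds to high score change and name input request events.
; Those events refresh the high score text or reveal name entry with UI focus.
; Tick rewrites the score text every frame, leaving it blank unless the score is positive.
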(event `self.ReceiveBeginPlay`
  (bind _returnvalue (`GameplayStatics.GetPlayerControllerFromID` 0))
  (bind _returnvalue_2 (`|CreateWidget` "/Game/Widgets/W_CurrentScore.W_CurrentScore_C" _returnvalue))
  (bind _output_get (set `self.ScoreWidget` _returnvalue_2))
  (`UserWidget.AddToViewport` _output_get 0)
  (bind _returnvalue_3 (`|CreateWidget` "/Game/Widgets/W_HighScores.W_HighScores_C" _returnvalue))
  (bind _output_get_2 (set `self.HighScoreWidget` _returnvalue_3))
  (`UserWidget.AddToViewport` _output_get_2 0)
  (add `self.OnHighScoreChange` (delegate `UpdateHighScore`))
  (`self.UpdateHighScore`)
  (bind _returnvalue_4 (`|CreateWidget` "/Game/Widgets/W_NameInput.W_NameInput_C" _returnvalue))
  (bind _output_get_3 (set `self.NameInputWidget` _returnvalue_4))
  (`UserWidget.AddToViewport` _output_get_3 0)
  (`Widget.SetVisibility` _output_get_3 "Hidden")
  (add `self.OnRequestNameInput` (delegate `RequestNameInput`)))

(event `UpdateHighScore`
  (bind _asbp_endless_game_state (cast `/Game/BP_EndlessGameState` (`GameplayStatics.GetGameState`)))
  (bind _returnvalue (`self.GetHighScoreString` _asbp_endless_game_state))
  (set `/Game/Widgets/W_HighScores.HighScoreString` _returnvalue (`self.HighScoreWidget`)))

(event `RequestNameInput`
  (bind _returnvalue (`GameplayStatics.GetPlayerControllerFromID` 0))
  (bind _nameinputwidget (`self.NameInputWidget`))
  (`Widget.SetVisibility` _nameinputwidget "Visible")
  (`WidgetBlueprintLibrary.SetInputMode_GameAndUIEx` _returnvalue _nameinputwidget)
  (`Widget.SetUserFocus` (`/Game/Widgets/W_NameInput.EditableTextBox_46` _nameinputwidget) _returnvalue))

(event `self.ReceiveTick`
  (params (DeltaSeconds :type "Float (single-precision)"))
  (bind _currentscore (`self.CurrentScore`))
  (bind _scorewidget (`self.ScoreWidget`))
  (`/Engine/EditorBlueprintResources/StandardMacros.CompareInt` _currentscore
    (:`>`
      (set `/Game/Widgets/W_CurrentScore.ScoreString` (`KismetStringLibrary.Concat_StrStr` "Score: " (`KismetStringLibrary.Conv_IntToString` _currentscore)) _scorewidget))
    (:`==`
      (set `/Game/Widgets/W_CurrentScore.ScoreString` "" _scorewidget :!label _label))
    (:`<`
      (goto _label))))

(fn `UserConstructionScript`)